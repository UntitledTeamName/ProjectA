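; Player character Blueprint with first/third-person view switching, crouch and prone camera heights, and rifle aim-down-sights.
; BeginPlay creates the crosshair and attaches a spawned rifle to the first-person arms, hiding crosshair and arms until view toggles.
; Timelines lower the FPP camera and blend the arms toward an ADS pose computed by inverting the rifle's AimPoint socket transform.
; CanProne is unfinished and uncalled, AttachWeapon is empty, and stance flags are never set here.
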(event `EnhancedInput|/Game/ProjectA/Input/Actions/IA_Prone`
  (params (ActionValue :type Boolean) (ElapsedSeconds :type "Float (double-precision)") (TriggeredSeconds :type "Float (double-precision)") (InputAction :type "InputAction Object Reference" :default "/Game/ProjectA/Input/Actions/IA_Prone.IA_Prone"))
  (bind _cameraheight (`self.CameraHeight`))
  (:`Started`
    (if (`self.bIsCrouched`)
      _
      (elif (`self.bIsProning`)
        (bind (_direction _offeset_value) (`Timeline|Prone Height` :!via `ReverseFromEnd` :!label _label)
          (:`Update`
            (`SceneComponent.K2_SetRelativeLocation` (`self.FPPCamera`) (`KismetMathLibrary.MakeVector` 0.0 0.0 (- _cameraheight (* (/ _cameraheight 1.5) _offeset_value))) false false)))
        (else
          (goto _label :!via `PlayFromStart`))))))

(event `EnhancedInput|/Game/ProjectA/Input/Actions/IA_Crouch`
  (params (ActionValue :type Boolean) (ElapsedSeconds :type "Float (double-precision)") (TriggeredSeconds :type "Float (double-precision)") (InputAction :type "InputAction Object Reference" :default "/Game/ProjectA/Input/Actions/IA_Crouch.IA_Crouch"))
  (bind _cameraheight (`self.CameraHeight`))
  (:`Started`
    (if (`self.bIsProning`)
      _
      (elif (`self.bIsCrouched`)
        (bind (_direction _offeset_value) (`Timeline|Crouch Height` :!via `ReverseFromEnd` :!label _label_2)
          (:`Update`
            (`SceneComponent.K2_SetRelativeLocation` (`self.FPPCamera`) (`KismetMathLibrary.MakeVector` 0.0 0.0 (- _cameraheight (* _offeset_value (/ _cameraheight 2.0)))) false false)))
        (else
          (goto _label_2 :!via `PlayFromStart`))))))

(event `EnhancedInput|/Game/ProjectA/Input/Actions/IA_ChangeView`
  (params (ActionValue :type Boolean) (ElapsedSeconds :type "Float (double-precision)") (TriggeredSeconds :type "Float (double-precision)") (InputAction :type "InputAction Object Reference" :default "/Game/ProjectA/Input/Actions/IA_ChangeView.IA_ChangeView"))
  (bind _tppcamera (`self.TPPCamera`))
  (bind _fppcamera (`self.FPPCamera`))
  (bind _fpparms (`self.FPPArms`))
  (bind _bp_crosshair (`self.BP_Crosshair`))
  (:`Started`
    (if (`self.bIsFPP`)
      (set `self.bIsFPP` false)
      (`ActorComponent.SetActive` _fppcamera false false)
      (`ActorComponent.SetActive` _tppcamera true false)
      (`SceneComponent.SetVisibility` (`self.Mesh`) true false)
      (`Widget.SetVisibility` _bp_crosshair "Hidden")
      (`SceneComponent.SetVisibility` _fpparms false true)
      (else
        (set `self.bIsFPP` true)
        (`ActorComponent.SetActive` _fppcamera true false)
        (`ActorComponent.SetActive` _tppcamera false false)
        (`SceneComponent.SetVisibility` (`self.Mesh`) false false)
        (`Widget.SetVisibility` _bp_crosshair "Visible")
        (`SceneComponent.SetVisibility` _fpparms true true)))))

(event `self.ReceiveBeginPlay`
  (bind _bp_crosshair (`self.BP_Crosshair`))
  (bind (_relativelocation_x _relativelocation_y _relativelocation_z) (`KismetMathLibrary.BreakVector` (`SceneComponent.RelativeLocation` (`self.FPPCamera`))))
  (set `self.CameraHeight` _relativelocation_z)
  (bind _returnvalue (`|GenericCreateObject` "/Game/ProjectA/Blueprints/UI/WBP_Crosshair.WBP_Crosshair_C"))
  (set `self.BP_Crosshair` _returnvalue)
  (`UserWidget.AddToViewport` _bp_crosshair 0)
  (`Widget.SetVisibility` _bp_crosshair "Hidden")
  (set `self.DefaultsArmsTransform` (`SceneComponent.GetRelativeTransform` (`self.FPPArms`)))
  (bind _returnvalue_2 (`|SpawnActorFromClass` "/Game/ProjectA/Blueprints/Weapon/BP_Rifle.BP_Rifle_C" (`self.DefaultsArmsTransform`) "Undefined" "MultiplyWithRoot" null null))
  (bind _output_get (set `self.BP_Rifle` _returnvalue_2))
  (`self.K2_AttachToComponent` _output_get (`self.FPPArms`) "GripPoint" "SnapToTarget" "SnapToTarget" "SnapToTarget" true)
  (`SceneComponent.SetVisibility` (`self.FPPArms`) false true))

(event `EnhancedInput|/Game/ProjectA/Input/Actions/IA_Aim`
  (params (ActionValue :type Boolean) (ElapsedSeconds :type "Float (double-precision)") (TriggeredSeconds :type "Float (double-precision)") (InputAction :type "InputAction Object Reference" :default "/Game/ProjectA/Input/Actions/IA_Aim.IA_Aim"))
  (:`Triggered`
    (set `self.bIsAiming` true)
    (bind (_direction _newtrack_0) (`Timeline|Timeline` :!label _label_3)
      (:`Update`
        (`SceneComponent.K2_SetRelativeTransform` (`self.FPPArms`) (`KismetMathLibrary.TLerp` (`KismetMathLibrary.SelectTransform` (`SceneComponent.GetRelativeTransform` (`self.FPPArms`)) (`self.DefaultsArmsTransform`) (`self.bIsAiming`)) (`self.CalculateADSTransform`) _newtrack_0) false false))))
  (:`Completed`
    (set `self.bIsAiming` false)
    (goto _label_3 :!via `ReverseFromEnd`)))

(fn `AttachWeapon`)

(fn `CalculateADSTransform`
  (returns (ReturnValue :type "Transform Structure"))
  (return (`KismetMathLibrary.MakeTransform` (`KismetMathLibrary.MakeVector` (+ (.x (.location (`KismetMathLibrary.InvertTransform` (`KismetMathLibrary.MakeRelativeTransform` (`SceneComponent.GetSocketTransform` (`/Game/ProjectA/Blueprints/Weapon/BP_Rifle.Mesh` (`self.BP_Rifle`)) "AimPoint" "RTS_World") (`SceneComponent.K2_GetComponentToWorld` (`self.FPPArms`)))))) 20.0) (.y (.location (`KismetMathLibrary.InvertTransform` (`KismetMathLibrary.MakeRelativeTransform` (`SceneComponent.GetSocketTransform` (`/Game/ProjectA/Blueprints/Weapon/BP_Rifle.Mesh` (`self.BP_Rifle`)) "AimPoint" "RTS_World") (`SceneComponent.K2_GetComponentToWorld` (`self.FPPArms`)))))) (.z (.location (`KismetMathLibrary.InvertTransform` (`KismetMathLibrary.MakeRelativeTransform` (`SceneComponent.GetSocketTransform` (`/Game/ProjectA/Blueprints/Weapon/BP_Rifle.Mesh` (`self.BP_Rifle`)) "AimPoint" "RTS_World") (`SceneComponent.K2_GetComponentToWorld` (`self.FPPArms`))))))) (.rotation (`KismetMathLibrary.InvertTransform` (`KismetMathLibrary.MakeRelativeTransform` (`SceneComponent.GetSocketTransform` (`/Game/ProjectA/Blueprints/Weapon/BP_Rifle.Mesh` (`self.BP_Rifle`)) "AimPoint" "RTS_World") (`SceneComponent.K2_GetComponentToWorld` (`self.FPPArms`))))) (.scale (`KismetMathLibrary.InvertTransform` (`KismetMathLibrary.MakeRelativeTransform` (`SceneComponent.GetSocketTransform` (`/Game/ProjectA/Blueprints/Weapon/BP_Rifle.Mesh` (`self.BP_Rifle`)) "AimPoint" "RTS_World") (`SceneComponent.K2_GetComponentToWorld` (`self.FPPArms`))))))))

(fn `Can Prone`
  (returns (`Yes/No` :type Boolean) (`Adjusted Location` :type "Vector Structure"))
  (bind _returnvalue (+ (`self.K2_GetActorLocation`) (0.0 0.0 -50.0)))
  (bind _returnvalue_2 (+ (`self.K2_GetActorLocation`) (0.0 0.0 -50.0)))
  (`KismetSystemLibrary.SphereTraceMulti` :`Start` _returnvalue_2 :`End` (+ _returnvalue_2 (* (`self.GetActorForwardVector`) 80.0)) :`Radius` 30.0 :`TraceChannel` "TraceTypeQuery1" :`DrawDebugType` "ForDuration")
  (`KismetSystemLibrary.SphereTraceMulti` :`Start` _returnvalue :`End` (+ _returnvalue (* (`self.GetActorForwardVector`) -80.0)) :`Radius` 30.0 :`TraceChannel` "TraceTypeQuery1" :`DrawDebugType` "ForDuration"))

(fn `UserConstructionScript`)